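; BP_RPGController is a player controller that owns the player's HUD and shows pickup-name messages on it.
; On BeginPlay it waits briefly, then creates W_PlayerUI and adds it to the viewport, only for the local controller.
; ShowPickupName relays a name and state through ClientShowPickup to the widget's PlayerMessage function.
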(event Custom|ClientShowPickup
  (params (State :type Boolean) (Message :type Text))
  (Default|PlayerMessage (Variables|Default|GetPlayerUI) State Message))

(event EventShowPickupName
  (params (Name :type Text) (State :type Boolean))
  (CallFunction|ClientShowPickup State Name))

(event EventBeginPlay
  ;[1 1 1] UI stuff
  (Utilities|FlowControl|Delay 0.2)
  (if (Pawn|IsLocalPlayerController)
    (bind _returnvalue (UserInterface|CreateWidget "/Game/_Main/UI/W_PlayerUI.W_PlayerUI_C"))
    (bind _output_get (Variables|Default|SetPlayerUI _returnvalue))
    (UserInterface|Viewport|AddtoViewport _output_get 0)))

(fn ConstructionScript)