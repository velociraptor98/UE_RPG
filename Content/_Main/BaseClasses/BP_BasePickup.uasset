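; Base pickup actor with a physics-simulated static mesh and a sphere trigger for detecting nearby players.
; On the authority only, sphere overlap begin and end tell actors tagged Player to show or clear pickup info for this actor via SetPickupInfoMessage.
; DisablePhysics turns off simulation and collision on mesh and sphere, and GetPickupType exposes the type from PickupInfo.
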(event OnComponentEndOverlap(Sphere)
  (params (OverlappedComponent :type Primitive%20Component%20Object%20Reference) (OtherActor :type Actor%20Object%20Reference) (OtherComp :type Primitive%20Component%20Object%20Reference) (OtherBodyIndex :type Integer))
  (Networking|SwitchHasAuthority
    (:Authority
      (if (Actor|ActorHasTag OtherActor "Player")
        (Class|BPIHeroChar|SetPickupInfo(Message) OtherActor self false)))))

(event OnComponentBeginOverlap(Sphere)
  (params (OverlappedComponent :type Primitive%20Component%20Object%20Reference) (OtherActor :type Actor%20Object%20Reference) (OtherComp :type Primitive%20Component%20Object%20Reference) (OtherBodyIndex :type Integer) (bFromSweep :type Boolean) (SweepResult :type Hit%20Result%20Structure%20%28by%20ref%29))
  (Networking|SwitchHasAuthority
    (:Authority
      (if (Actor|ActorHasTag OtherActor "Player")
        (Class|BPIHeroChar|SetPickupInfo(Message) OtherActor self true)))))

(event EventBeginPlay
  (Physics|SetSimulatePhysics (Variables|Default|GetStaticMesh) true))

(event EventDisablePhysics
  (Physics|SetSimulatePhysics (Variables|Default|GetStaticMesh) false)
  (Collision|SetCollisionEnabled (Variables|Default|GetSphere) "NoCollision"))

(fn ConstructionScript)

(fn GetPickupType
  (return (.PickupType (Utilities|Struct|BreakStruct_PickupInfo (Variables|Default|GetPickupInfo)))))